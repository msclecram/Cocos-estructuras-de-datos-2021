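; Ball1 is a Blueprint that tallies points from two goals and passes the total to the score HUD.
; On BeginPlay it binds a handler to each goal's event dispatcher, and each handler adds that goal's Score to its own running subtotal.
; Both handlers then sum the subtotals and write the result to ScoreNew on the referenced ScoreHUD, with the same write wired to the failed-cast branch.
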(event `self.ReceiveBeginPlay`
  (add `/Game/Goal/Goal.Entrada al Evento` (`self.OtherGoal`) (delegate `HasEnter`))
  (add `/Game/Goal/Goal1.Entrada al Evento2` (`self.OtherGoal2`) (delegate `CustomEvent_0`)))

(event `HasEnter`
  (bind _output_get (set `self.TotalScoreR` (+ (`self.TotalScoreR`) (`/Game/Goal/Goal.Score` (`self.OtherGoal`)))))
  (bind _output_get_2 (set `self.TotalScore` (+ _output_get (stale `CustomEvent_0` _output_get)) :!label _label))
  (bind _asscore_hud (cast `/Game/VehicleCPP/ScoreHUD` (`self.ScoreHud`))
    (:`then`
      (set `/Game/VehicleCPP/ScoreHUD.ScoreNew` _output_get_2 _asscore_hud))
    (:`CastFailed`
      (set `/Game/VehicleCPP/ScoreHUD.ScoreNew` _output_get_2 _asscore_hud))))

(event `CustomEvent_0`
  (bind _output_get (set `self.TotalScoreR2` (+ (`self.TotalScoreR2`) (`/Game/Goal/Goal1.Score` (`self.OtherGoal2`)))))
  (goto _label))

(fn `NewFunction_0`)

(fn `UserConstructionScript`)